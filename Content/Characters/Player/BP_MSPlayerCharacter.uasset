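; Player character Blueprint with debug keys for testing damage and healing through the Gameplay Ability System.
; V and C call server-named events that build GE_Damage and GE_Healing specs with the character as effect causer.
; Each spec receives a fixed, tag-based SetByCaller health magnitude, then is applied to the character's own AbilitySystemComponent.
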(event Custom|Server_ApplyDamageEffect
  (bind _returnvalue (Spec|MakeSpecHandle(ByClass) "/Game/Effects/GameplayEffects/GE_Damage.GE_Damage_C" 0 self))
  (bind _returnvalue_2 (Ability|GameplayEffect|AssignTagSetbyCallerMagnitude _returnvalue "(TagName=\"Data.Health.ConsumptionAmount\")" -3e+01))
  (GameplayEffects|ApplyGameplayEffectSpecToSelf (Variables|Default|GetAbilitySystemComponent) _returnvalue_2))

(event Custom|Server_ApplyHealEffect
  (bind _returnvalue (Spec|MakeSpecHandle(ByClass) "/Game/Effects/GameplayEffects/GE_Healing.GE_Healing_C" 0 self))
  (bind _returnvalue_2 (Ability|GameplayEffect|AssignTagSetbyCallerMagnitude _returnvalue "(TagName=\"Data.Health.GainedAmount\")" 3e+01))
  (GameplayEffects|ApplyGameplayEffectSpecToSelf (Variables|Default|GetAbilitySystemComponent) _returnvalue_2))

(event EventBeginPlay)

(event Collision|EventActorBeginOverlap
  (params (OtherActor :type Actor%20Object%20Reference)))

(event EventTick
  (params (DeltaSeconds :type Float%20%28single-precision%29)))

(event Input|KeyboardEvents|DebugKeyC
  (params (Key :type Key%20Structure :default "None") (ActionValue :type Input%20Action%20Value%20Structure))
  (:Pressed
    (CallFunction|ServerApplyHealEffect)))

(event Input|KeyboardEvents|DebugKeyV
  (params (Key :type Key%20Structure :default "None") (ActionValue :type Input%20Action%20Value%20Structure))
  (:Pressed
    (CallFunction|ServerApplyDamageEffect)))

(fn ConstructionScript)